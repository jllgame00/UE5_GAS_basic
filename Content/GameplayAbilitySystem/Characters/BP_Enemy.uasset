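; BP_Enemy is an enemy character Blueprint that uses the Gameplay Ability System to handle its death.
; On BeginPlay it grants GA_Dead to its AbilitySystemComponent and starts a fast looping timer on CheckDeadTag.
; CheckDeadTag polls the State.Dead tag count rather than listening for tag events.
; Once the tag is present, it tries to activate GA_Dead and clears the timer.
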(event `self.ReceiveBeginPlay`
  (`AbilitySystemComponent.K2_GiveAbility` (`self.AbilitySystemComponent`) "/Game/GameplayAbilitySystem/Abilities/GA_Dead.GA_Dead_C" 1 -1)
  (`KismetSystemLibrary.K2_SetTimer` null "CheckDeadTag" 0.05 true))

(fn `CheckDeadTag`
  (if (> (`AbilitySystemComponent.GetGameplayTagCount` (`self.AbilitySystemComponent`) (struct :`TagName` "State.Dead")) 0)
    (`AbilitySystemComponent.TryActivateAbilityByClass` (`self.AbilitySystemComponent`) "/Game/GameplayAbilitySystem/Abilities/GA_Dead.GA_Dead_C" true)
    (`KismetSystemLibrary.K2_ClearTimer` null "CheckDeadTag")))

(fn `UserConstructionScript`)